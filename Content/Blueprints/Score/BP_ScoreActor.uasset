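; BP_ScoreActor is a goal trigger for a paddle-and-ball game that awards a point when a ball enters it.
; On BeginPlay it caches player 0's BP_Paddle pawn to reach that paddle's score widget.
; When a BP_Ball overlaps its collision box, it destroys the ball and updates Player 1's or Player 2's score on the widget, chosen by the Player1Goal flag.
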(event `self.ReceiveBeginPlay`
  (bind _asbp_paddle (cast `/Game/Blueprints/Paddles/BP_Paddle` (`GameplayStatics.GetPlayerPawn` 0)))
  (set `self.PaddleRef` _asbp_paddle))

(event `self.BoxCollision.OnComponentBeginOverlap`
  (params (OverlappedComponent :type "PrimitiveComponent Object Reference") (OtherActor :type "Actor Object Reference") (OtherComp :type "PrimitiveComponent Object Reference") (OtherBodyIndex :type Integer) (bFromSweep :type Boolean) (SweepResult :type "HitResult Structure (by ref)"))
  (bind _widgetrefscore (`/Game/Blueprints/Paddles/BP_Paddle.WidgetRefScore` (`self.PaddleRef`)))
  (bind _asbp_ball (cast `/Game/Blueprints/Ball/BP_Ball` OtherActor))
  (`self.K2_DestroyActor` _asbp_ball)
  (if (`self.Player1Goal`)
    (`/Game/Widget/WB_Score.Update Player 1 Score` _widgetrefscore)
    (else
      (`/Game/Widget/WB_Score.Update Player 2 Score` _widgetrefscore))))

(fn `UserConstructionScript`)