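; BP_Ball is a physics-driven ball that launches itself along negative X when play begins.
; On BeginPlay it finds the AI_BP actor, registers itself as that actor's BallRef, and applies a velocity-change impulse to its Sphere.
; On each hit it clamps the velocity's magnitude to exactly BallSpeed, keeping a constant speed through bounces.
; The per-hit BallSpeed increment is zero, so the ball does not accelerate.
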(event `self.ReceiveBeginPlay`
  (bind _returnvalue (`GameplayStatics.GetActorOfClass` "/Game/Blueprints/Paddles/AI_BP.AI_BP_C"))
  (bind _output_get (set `self.AIRef` _returnvalue))
  (set `/Game/Blueprints/Paddles/AI_BP.BallRef` self _output_get)
  (`PrimitiveComponent.AddImpulse` (`self.Sphere`) (-1200.0 0.0 0.0) "None" true))

(event `self.ReceiveHit`
  (params (MyComp :type "PrimitiveComponent Object Reference") (Other :type "Actor Object Reference") (OtherComp :type "PrimitiveComponent Object Reference") (bSelfMoved :type Boolean) (HitLocation :type "Vector Structure") (HitNormal :type "Vector Structure") (NormalImpulse :type "Vector Structure") (Hit :type "HitResult Structure (by ref)"))
  (bind _ballspeed (`self.BallSpeed`))
  (bind _sphere (`self.Sphere`))
  (set `self.BallSpeed` (+ (`self.BallSpeed`) 0.0))
  (bind _returnvalue (`PrimitiveComponent.GetPhysicsLinearVelocity` _sphere "None"))
  (`PrimitiveComponent.SetPhysicsLinearVelocity` _sphere (`KismetMathLibrary.ClampVectorSize` _returnvalue _ballspeed _ballspeed) false "None")
  (`PrimitiveComponent.GetPhysicsLinearVelocity` (`self.Sphere`) "None"))

(fn `UserConstructionScript`)